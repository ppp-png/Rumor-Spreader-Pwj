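; Sci-fi light fixture decal actor with a matching RectLight and optional flicker.
; The construction script keeps either a masked plane or bordered/borderless decals, then configures dynamic materials and the light's size and source texture from type, variant and appearance settings.
; Curve-driven timelines flicker standby and RGB channels at separate rates and phases.
; The R timeline plays whenever any flicker is enabled, as its update alone drives emissive parameters and light color and intensity.
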(event EventBeginPlay
  (bind _timelineflickerb (Variables|Default|GetTimelineFlickerB))
  (bind _timelineflickerg (Variables|Default|GetTimelineFlickerG))
  (bind _timelineflickerr (Variables|Default|GetTimelineFlickerR))
  (bind _timelineflickerstandby (Variables|Default|GetTimelineFlickerStandby))
  (Components|Timeline|SetPlayRate _timelineflickerstandby (Variables|Flicker|GetFrequencyStandby))
  (Components|Timeline|SetPlayRate _timelineflickerr (Variables|Flicker|GetFrequencyR))
  (Components|Timeline|SetPlayRate _timelineflickerg (Variables|Flicker|GetFrequencyG))
  (Components|Timeline|SetPlayRate _timelineflickerb (Variables|Flicker|GetFrequencyB))
  (Components|Timeline|SetPlaybackPosition _timelineflickerstandby (Variables|Flicker|GetPhaseStandby) false true)
  (Components|Timeline|SetPlaybackPosition _timelineflickerr (Variables|Flicker|GetPhaseR) false true)
  (Components|Timeline|SetPlaybackPosition _timelineflickerg (Variables|Flicker|GetPhaseG) false true)
  (Components|Timeline|SetPlaybackPosition _timelineflickerb (Variables|Flicker|GetPhaseB) false true)
  (for _array_element (Utilities|Array|MakeArray (Math|Boolean|ORBoolean (Variables|Flicker|GetFlickerR) (Variables|Flicker|GetFlickerG) (Variables|Flicker|GetFlickerB) (Variables|Flicker|GetFlickerStandby)) (Variables|Flicker|GetFlickerG) (Variables|Flicker|GetFlickerB) (Variables|Flicker|GetFlickerStandby))
    (if _array_element
      (Audio|Components|Audio|Play (Utilities|Array|MakeArray (Variables|Default|GetTimelineFlickerR) (Variables|Default|GetTimelineFlickerG) (Variables|Default|GetTimelineFlickerB) (Variables|Default|GetTimelineFlickerStandby))))))

(fn ConstructionScript
  (bind _returnvalue (Transformation|GetActorRotation))
  (bind _emittervariant (Variables|Body|GetEmitterVariant))
  (bind _size (Variables|Body|GetSize))
  (bind _plane (Variables|Default|GetPlane))
  (bind _type (Variables|Body|GetType))
  (bind _monochrome (Variables|Light|GetMonochrome))
  (bind _texmask1 (Variables|Textures|GetTexMask1))
  (bind _texmask2 (Variables|Textures|GetTexMask2))
  (bind _texnormal1 (Variables|Textures|GetTexNormal1))
  (bind _texnormal2 (Variables|Textures|GetTexNormal2))
  (bind _texemissive1 (Variables|Textures|GetTexEmissive1))
  (bind _texemissive2 (Variables|Textures|GetTexEmissive2))
  (bind _rectlight (Variables|Default|GetRectLight))
  (bind _rectlight_2 (Variables|Default|GetRectLight))
  (bind _decal (Variables|Default|GetDecal))
  (bind _type_2 (Variables|Body|GetType))
  (bind (_x _y _z) (Math|Rotator|BreakRotIntoAxes _returnvalue))
  (bind _returnvalue_2 (> _monochrome 0.5))
  (bind _returnvalue_3 (/ _size 3e+01))
  (bind _returnvalue_4 (* _size 0.01))
  (bind _returnvalue_5 (Utilities|Select :Index _type_2 :Option%200 "(X=16.000000,Y=8.000000)" :Option%201 "(X=8.000000,Y=8.000000)" :Option%202 "(X=16.000000,Y=8.000000)" :Option%203 "(X=8.000000,Y=8.000000)"))
  (bind _returnvalue_6 (* _returnvalue_5 _returnvalue_3))
  (bind _returnvalue_7 (/ _returnvalue_4 3.0))
  (Transformation|SetWorldScale3D (Variables|Default|GetDecal) (Math|Vector|MakeVector 1.0 _returnvalue_7 _returnvalue_4))
  (Class|RectLightComponent|SetSourceWidth _rectlight (.x _returnvalue_6))
  (Class|RectLightComponent|SetSourceHeight _rectlight (.y _returnvalue_6))
  (Class|RectLightComponent|SetSourceTexture (Variables|Default|GetRectLight) (Utilities|Select :Index (Variables|Body|GetType) :Option%200 (select _returnvalue_2 (Utilities|Select :Index _emittervariant :Option%200 "/Game/SciFiLightSourceDecalsV01/Textures/LightSourceTexture00m.LightSourceTexture00m" :Option%201 "/Game/SciFiLightSourceDecalsV01/Textures/LightSourceTexture01m.LightSourceTexture01m" :Option%202 "/Game/SciFiLightSourceDecalsV01/Textures/LightSourceTexture02m.LightSourceTexture02m" :Option%203 "/Game/SciFiLightSourceDecalsV01/Textures/LightSourceTexture03m.LightSourceTexture03m" :Option%204 "/Game/SciFiLightSourceDecalsV01/Textures/LightSourceTexture04m.LightSourceTexture04m" :Option%205 "/Game/SciFiLightSourceDecalsV01/Textures/LightSourceTexture05m.LightSourceTexture05m") (Utilities|Select :Index _emittervariant :Option%200 "/Game/SciFiLightSourceDecalsV01/Textures/LightSourceTexture00.LightSourceTexture00" :Option%201 "/Game/SciFiLightSourceDecalsV01/Textures/LightSourceTexture01.LightSourceTexture01" :Option%202 "/Game/SciFiLightSourceDecalsV01/Textures/LightSourceTexture02.LightSourceTexture02" :Option%203 "/Game/SciFiLightSourceDecalsV01/Textures/LightSourceTexture03.LightSourceTexture03" :Option%204 "/Game/SciFiLightSourceDecalsV01/Textures/LightSourceTexture04.LightSourceTexture04" :Option%205 "/Game/SciFiLightSourceDecalsV01/Textures/LightSourceTexture05.LightSourceTexture05")) :Option%201 (select _returnvalue_2 (Utilities|Select :Index _emittervariant :Option%200 "/Game/SciFiLightSourceDecalsV01/Textures/LightSourceTexture10m.LightSourceTexture10m" :Option%201 "/Game/SciFiLightSourceDecalsV01/Textures/LightSourceTexture11m.LightSourceTexture11m" :Option%202 "/Game/SciFiLightSourceDecalsV01/Textures/LightSourceTexture12m.LightSourceTexture12m" :Option%203 "/Game/SciFiLightSourceDecalsV01/Textures/LightSourceTexture13m.LightSourceTexture13m" :Option%204 "/Game/SciFiLightSourceDecalsV01/Textures/LightSourceTexture14m.LightSourceTexture14m" :Option%205 "/Game/SciFiLightSourceDecalsV01/Textures/LightSourceTexture15m.LightSourceTexture15m") (Utilities|Select :Index _emittervariant :Option%200 "/Game/SciFiLightSourceDecalsV01/Textures/LightSourceTexture10.LightSourceTexture10" :Option%201 "/Game/SciFiLightSourceDecalsV01/Textures/LightSourceTexture11.LightSourceTexture11" :Option%202 "/Game/SciFiLightSourceDecalsV01/Textures/LightSourceTexture12.LightSourceTexture12" :Option%203 "/Game/SciFiLightSourceDecalsV01/Textures/LightSourceTexture13.LightSourceTexture13" :Option%204 "/Game/SciFiLightSourceDecalsV01/Textures/LightSourceTexture14.LightSourceTexture14" :Option%205 "/Game/SciFiLightSourceDecalsV01/Textures/LightSourceTexture15.LightSourceTexture15")) :Option%202 (select _returnvalue_2 (Utilities|Select :Index _emittervariant :Option%200 "/Game/SciFiLightSourceDecalsV01/Textures/LightSourceTexture20m.LightSourceTexture20m" :Option%201 "/Game/SciFiLightSourceDecalsV01/Textures/LightSourceTexture21m.LightSourceTexture21m" :Option%202 "/Game/SciFiLightSourceDecalsV01/Textures/LightSourceTexture22m.LightSourceTexture22m" :Option%203 "/Game/SciFiLightSourceDecalsV01/Textures/LightSourceTexture23m.LightSourceTexture23m" :Option%204 "/Game/SciFiLightSourceDecalsV01/Textures/LightSourceTexture24m.LightSourceTexture24m" :Option%205 "/Game/SciFiLightSourceDecalsV01/Textures/LightSourceTexture25m.LightSourceTexture25m") (Utilities|Select :Index _emittervariant :Option%200 "/Game/SciFiLightSourceDecalsV01/Textures/LightSourceTexture20.LightSourceTexture20" :Option%201 "/Game/SciFiLightSourceDecalsV01/Textures/LightSourceTexture21.LightSourceTexture21" :Option%202 "/Game/SciFiLightSourceDecalsV01/Textures/LightSourceTexture22.LightSourceTexture22" :Option%203 "/Game/SciFiLightSourceDecalsV01/Textures/LightSourceTexture23.LightSourceTexture23" :Option%204 "/Game/SciFiLightSourceDecalsV01/Textures/LightSourceTexture24.LightSourceTexture24" :Option%205 "/Game/SciFiLightSourceDecalsV01/Textures/LightSourceTexture25.LightSourceTexture25")) :Option%203 (select _returnvalue_2 (Utilities|Select :Index _emittervariant :Option%200 "/Game/SciFiLightSourceDecalsV01/Textures/LightSourceTexture30m.LightSourceTexture30m" :Option%201 "/Game/SciFiLightSourceDecalsV01/Textures/LightSourceTexture31m.LightSourceTexture31m" :Option%202 "/Game/SciFiLightSourceDecalsV01/Textures/LightSourceTexture32m.LightSourceTexture32m" :Option%203 "/Game/SciFiLightSourceDecalsV01/Textures/LightSourceTexture33m.LightSourceTexture33m" :Option%204 "/Game/SciFiLightSourceDecalsV01/Textures/LightSourceTexture34m.LightSourceTexture34m" :Option%205 "/Game/SciFiLightSourceDecalsV01/Textures/LightSourceTexture35m.LightSourceTexture35m") (Utilities|Select :Index _emittervariant :Option%200 "/Game/SciFiLightSourceDecalsV01/Textures/LightSourceTexture30.LightSourceTexture30" :Option%201 "/Game/SciFiLightSourceDecalsV01/Textures/LightSourceTexture31.LightSourceTexture31" :Option%202 "/Game/SciFiLightSourceDecalsV01/Textures/LightSourceTexture32.LightSourceTexture32" :Option%203 "/Game/SciFiLightSourceDecalsV01/Textures/LightSourceTexture33.LightSourceTexture33" :Option%204 "/Game/SciFiLightSourceDecalsV01/Textures/LightSourceTexture34.LightSourceTexture34" :Option%205 "/Game/SciFiLightSourceDecalsV01/Textures/LightSourceTexture35.LightSourceTexture35"))))
  (if (Variables|Body|GetMaskedMesh)
    (Transformation|SetWorldScale3D _plane (Math|Vector|MakeVector _returnvalue_4 _returnvalue_7 1.0))
    (Variables|Body|SetBorderless false)
    (Components|DestroyComponent (Variables|Default|GetDecalEmissive))
    (bind _returnvalue_8 (Rendering|Material|CreateDynamicMaterialInstance _plane 0 "/Game/SciFiLightSourceDecalsV01/Materials/LightMeshMaterial_Inst.LightMeshMaterial_Inst" "None" :!class /Script/Engine.PrimitiveComponent))
    (bind _output_get (Variables|Materials|SetMaterialE _returnvalue_8))
    (Variables|Materials|SetMaterialD _output_get)
    (else
      (Components|DestroyComponent _plane)
      (if (Variables|Body|GetBorderless)
        (bind _returnvalue_9 (Rendering|Material|CreateDynamicMaterialInstance (Variables|Default|GetDecalEmissive) :!class /Script/Engine.DecalComponent))
        (Variables|Materials|SetMaterialE _returnvalue_9)
        (Rendering|Components|Decal|SetDecalMaterial _decal "/Game/SciFiLightSourceDecalsV01/Materials/LightDecalBorderlessMaterial_Inst.LightDecalBorderlessMaterial_Inst")
        (bind _returnvalue_10 (Rendering|Material|CreateDynamicMaterialInstance (Variables|Default|GetDecal) :!class /Script/Engine.DecalComponent))
        (Variables|Materials|SetMaterialD _returnvalue_10)
        (else
          (Components|DestroyComponent (Variables|Default|GetDecalEmissive))
          (Rendering|Components|Decal|SetDecalMaterial _decal "/Game/SciFiLightSourceDecalsV01/Materials/LightDecalMaterial_Inst.LightDecalMaterial_Inst")
          (bind _returnvalue_11 (Rendering|Material|CreateDynamicMaterialInstance (Variables|Default|GetDecal) :!class /Script/Engine.DecalComponent))
          (bind _output_get_2 (Variables|Materials|SetMaterialD _returnvalue_11))
          (Variables|Materials|SetMaterialE _output_get_2)))))
  (bind _returnvalue_12 (Rendering|Material|CreateDynamicMaterialInstance (Variables|Default|GetDecalNormal) :!class /Script/Engine.DecalComponent))
  (bind _output_get_3 (Variables|Materials|SetMaterialN _returnvalue_12))
  (Rendering|Material|SetVectorParameterValue (Variables|Materials|GetMaterialE) "VariantV3" (Utilities|Struct|MakeLinearColor (Math|Conversions|ToFloat(Byte) (Variables|Body|GetBodyVariant)) (Math|Conversions|ToFloat(Byte) (Variables|Body|GetEmitterVariant)) (Utilities|Select :Index _type :Option%200 0.0 :Option%201 0.5 :Option%202 0.0 :Option%203 0.5) (Utilities|Select :Index _type :Option%200 3.56 :Option%201 8.0 :Option%202 3.95 :Option%203 6.2)) :!class /Script/Engine.MaterialInstanceDynamic)
  (Rendering|Material|SetScalarParameterValue (Variables|Materials|GetMaterialD) "Cutout" (select (Variables|Body|GetBorderless) -0.75 -0.25) :!class /Script/Engine.MaterialInstanceDynamic)
  (Rendering|Material|SetScalarParameterValue (Variables|Materials|GetMaterialN) "Cutout" (select (Variables|Body|GetBorderless) -0.5 0.0) :!class /Script/Engine.MaterialInstanceDynamic)
  (Rendering|Material|SetTextureParameterValue (Variables|Materials|GetMaterialD) "Mask" (Utilities|Select :Index _type :Option%200 _texmask1 :Option%201 _texmask1 :Option%202 _texmask2 :Option%203 _texmask2))
  (Rendering|Material|SetTextureParameterValue _output_get_3 "Normal" (Utilities|Select :Index _type :Option%200 _texnormal1 :Option%201 _texnormal1 :Option%202 _texnormal2 :Option%203 _texnormal2))
  (Rendering|Material|SetTextureParameterValue (Variables|Materials|GetMaterialD) "Emissive" (Utilities|Select :Index _type :Option%200 _texemissive1 :Option%201 _texemissive1 :Option%202 _texemissive2 :Option%203 _texemissive2))
  (Rendering|Material|SetVectorParameterValue (Variables|Materials|GetMaterialE) "EmissiveColor" (* (Variables|Light|GetEmissiveColor) (Variables|Light|GetEmissiveIntensity)) :!class /Script/Engine.MaterialInstanceDynamic)
  (Rendering|Material|SetVectorParameterValue (Variables|Materials|GetMaterialE) "EmissiveColorStandby" (* (Variables|Light|GetEmissiveColorStandby) (Variables|Light|GetEmissiveIntensityStandby)) :!class /Script/Engine.MaterialInstanceDynamic)
  (Rendering|Material|SetVectorParameterValue (Variables|Materials|GetMaterialD) "EmissiveComponents" (* (Variables|Light|GetEmissiveComponentFactor) (Variables|Light|GetEmissiveIntensity)) :!class /Script/Engine.MaterialInstanceDynamic)
  (Rendering|Material|SetVectorParameterValue (Variables|Materials|GetMaterialN) "X" (Math|Conversions|ToLinearColor(Vector) _x) :!class /Script/Engine.MaterialInstanceDynamic)
  (Rendering|Material|SetVectorParameterValue (Variables|Materials|GetMaterialN) "Y" (Math|Conversions|ToLinearColor(Vector) _y) :!class /Script/Engine.MaterialInstanceDynamic)
  (Rendering|Material|SetVectorParameterValue (Variables|Materials|GetMaterialN) "Z" (Math|Conversions|ToLinearColor(Vector) _z) :!class /Script/Engine.MaterialInstanceDynamic)
  (Rendering|Material|SetScalarParameterValue (Variables|Materials|GetMaterialD) "BodyMetallic" (Variables|Material|GetBodyMetallic) :!class /Script/Engine.MaterialInstanceDynamic)
  (Rendering|Material|SetScalarParameterValue (Variables|Materials|GetMaterialD) "BodyRoughness" (Variables|Material|GetBodyRoughness) :!class /Script/Engine.MaterialInstanceDynamic)
  (Rendering|Material|SetScalarParameterValue (Variables|Materials|GetMaterialD) "EmitterMetallic" (Variables|Material|GetEmitterMetallic) :!class /Script/Engine.MaterialInstanceDynamic)
  (Rendering|Material|SetScalarParameterValue (Variables|Materials|GetMaterialD) "EmitterRoughness" (Variables|Material|GetEmitterRoughness) :!class /Script/Engine.MaterialInstanceDynamic)
  (Rendering|Material|SetScalarParameterValue (Variables|Materials|GetMaterialD) "ScratchMetallic" (Variables|Material|GetScratchMetallic) :!class /Script/Engine.MaterialInstanceDynamic)
  (Rendering|Material|SetScalarParameterValue (Variables|Materials|GetMaterialD) "ScratchRoughness" (Variables|Material|GetScratchRoughness) :!class /Script/Engine.MaterialInstanceDynamic)
  (Rendering|Material|SetVectorParameterValue (Variables|Materials|GetMaterialD) "BodyColor" (Variables|Material|GetBodyColor) :!class /Script/Engine.MaterialInstanceDynamic)
  (Rendering|Material|SetVectorParameterValue (Variables|Materials|GetMaterialD) "EmitterColor" (Variables|Material|GetEmitterColor) :!class /Script/Engine.MaterialInstanceDynamic)
  (Rendering|Material|SetVectorParameterValue (Variables|Materials|GetMaterialD) "ScratchColor" (Variables|Material|GetScratchColor) :!class /Script/Engine.MaterialInstanceDynamic)
  (Rendering|Material|SetVectorParameterValue (Variables|Materials|GetMaterialD) "DustColor" (Variables|Material|GetDustColor) :!class /Script/Engine.MaterialInstanceDynamic)
  (Rendering|Material|SetScalarParameterValue (Variables|Materials|GetMaterialE) "Monochrome" (Variables|Light|GetMonochrome) :!class /Script/Engine.MaterialInstanceDynamic)
  (Rendering|Material|SetScalarParameterValue (Variables|Materials|GetMaterialD) "ScratchIntensity" (Variables|Material|GetScratchIntensity) :!class /Script/Engine.MaterialInstanceDynamic)
  (Rendering|Material|SetScalarParameterValue (Variables|Materials|GetMaterialD) "DustIntensity" (Variables|Material|GetDustIntensity) :!class /Script/Engine.MaterialInstanceDynamic)
  (Rendering|Components|Light|SetLightColor _rectlight_2 (Variables|Light|GetEmissiveColor) true)
  (Rendering|Components|Light|SetIntensity _rectlight_2 (* (Variables|Light|GetEmissiveIntensity) (Variables|Light|GetLightIntensityFactor)))
  (Class|TimelineComponent|SetFloatCurve (Variables|Default|GetTimelineFlickerStandby) (Variables|Flicker|GetFlickerCurveStandby) "Flicker01")
  (Class|TimelineComponent|SetFloatCurve (Variables|Default|GetTimelineFlickerR) (Variables|Flicker|GetFlickerCurveR) "Flicker01")
  (Class|TimelineComponent|SetFloatCurve (Variables|Default|GetTimelineFlickerG) (Variables|Flicker|GetFlickerCurveG) "Flicker01")
  (Class|TimelineComponent|SetFloatCurve (Variables|Default|GetTimelineFlickerB) (Variables|Flicker|GetFlickerCurveB) "Flicker01"))