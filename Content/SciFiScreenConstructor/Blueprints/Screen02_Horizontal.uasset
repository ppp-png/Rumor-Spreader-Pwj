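; Modular horizontal sci-fi screen prop, built entirely in the construction script.
; Width, Offset and left/right lengths position frame pieces, pick end/corner meshes and add repeated segments, with selectable grilles, fans, illumination and tilt angle.
; Front and flippable back screens scale to fit; unless stretched, a dynamic material instance corrects display UVs for aspect ratio, tiling and offset.
; A final pass applies BaseMaterial to every non-screen mesh component.
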(event EventBeginPlay)

(event Collision|EventActorBeginOverlap
  (params (OtherActor :type Actor%20Object%20Reference)))

(event EventTick
  (params (DeltaSeconds :type Float%20%28single-precision%29)))

(fn ConstructionScript
  (bind _grille1 (Variables|Default|GetGrille1))
  (bind _componentg1 (Variables|Default|GetComponentG1))
  (bind _displaymaterial (Variables|Default|GetDisplayMaterial))
  (bind _componentg2 (Variables|Default|GetComponentG2))
  (bind _screenbacksideflipy (Variables|Default|GetScreenBackSideFlipY))
  (bind _grille2 (Variables|Default|GetGrille2))
  (bind _componentg1_2 (Variables|Default|GetComponentG1))
  (bind _componentg2_2 (Variables|Default|GetComponentG2))
  (bind _illumination1 (Variables|Default|GetIllumination1))
  (bind _componentscreen (Variables|Default|GetComponentScreen))
  (bind _illumination1_2 (Variables|Default|GetIllumination1))
  (bind _illumination2 (Variables|Default|GetIllumination2))
  (bind _illumination2_2 (Variables|Default|GetIllumination2))
  (bind _illumination1_3 (Variables|Default|GetIllumination1))
  (bind _illumination2_3 (Variables|Default|GetIllumination2))
  (bind _screenmaterialoffset (Variables|Default|GetScreenMaterialOffset))
  (bind _lengthleft (Variables|Default|GetLengthLeft))
  (bind _screenbacksideflipx (Variables|Default|GetScreenBackSideFlipX))
  (bind _illumination1_4 (Variables|Default|GetIllumination1))
  (bind _illumination2_4 (Variables|Default|GetIllumination2))
  (bind _component2 (Variables|Default|GetComponent2))
  (bind _width (Variables|Default|GetWidth))
  (bind _width_2 (Variables|Default|GetWidth))
  (bind _width_3 (Variables|Default|GetWidth))
  (bind _offset (Variables|Default|GetOffset))
  (bind _width_4 (Variables|Default|GetWidth))
  (bind _returnvalue (== _lengthleft -1))
  (bind _returnvalue_2 (== _lengthleft 0))
  (bind _returnvalue_3 (== _lengthleft 1))
  (bind _returnvalue_4 (* _lengthleft 4e+01))
  (bind _returnvalue_5 (+ _width 8.0))
  (bind _returnvalue_6 (* _screenmaterialoffset -1.0))
  (bind _returnvalue_7 (* _width_3 1.0))
  (bind _returnvalue_8 (* _width_3 -0.5))
  (bind _returnvalue_9 (Utilities|Select :Index _grille2 :Option%200 "/Game/SciFiScreenConstructor/Meshes/Screen02_GrilleS01.Screen02_GrilleS01" :Option%201 "/Game/SciFiScreenConstructor/Meshes/Screen02_GrilleS02.Screen02_GrilleS02" :Option%202 "/Game/SciFiScreenConstructor/Meshes/Screen02_GrilleS03.Screen02_GrilleS03" :Option%203 "/Game/SciFiScreenConstructor/Meshes/Screen02_GrilleS04.Screen02_GrilleS04"))
  (bind _returnvalue_10 (select _illumination2_3 "/Game/SciFiScreenConstructor/Meshes/Screen02_FrameCC02.Screen02_FrameCC02" "/Game/SciFiScreenConstructor/Meshes/Screen02_FrameCC01.Screen02_FrameCC01"))
  (bind _returnvalue_11 (select _illumination1 "/Game/SciFiScreenConstructor/Meshes/Screen02_FrameS02.Screen02_FrameS02" "/Game/SciFiScreenConstructor/Meshes/Screen02_FrameS01.Screen02_FrameS01"))
  (bind _returnvalue_12 (Utilities|Select :Index _grille1 :Option%200 "/Game/SciFiScreenConstructor/Meshes/Screen02_GrilleS01.Screen02_GrilleS01" :Option%201 "/Game/SciFiScreenConstructor/Meshes/Screen02_GrilleS02.Screen02_GrilleS02" :Option%202 "/Game/SciFiScreenConstructor/Meshes/Screen02_GrilleS03.Screen02_GrilleS03" :Option%203 "/Game/SciFiScreenConstructor/Meshes/Screen02_GrilleS04.Screen02_GrilleS04"))
  (bind _returnvalue_13 (select _illumination2_4 "/Game/SciFiScreenConstructor/Meshes/Screen02_FrameCT02.Screen02_FrameCT02" "/Game/SciFiScreenConstructor/Meshes/Screen02_FrameCT01.Screen02_FrameCT01"))
  (bind _returnvalue_14 (select _illumination1_4 "/Game/SciFiScreenConstructor/Meshes/Screen02_FrameCC02.Screen02_FrameCC02" "/Game/SciFiScreenConstructor/Meshes/Screen02_FrameCC01.Screen02_FrameCC01"))
  (bind _returnvalue_15 (select _illumination1_3 "/Game/SciFiScreenConstructor/Meshes/Screen02_FrameCT02.Screen02_FrameCT02" "/Game/SciFiScreenConstructor/Meshes/Screen02_FrameCT01.Screen02_FrameCT01"))
  (bind _returnvalue_16 (select _illumination2 "/Game/SciFiScreenConstructor/Meshes/Screen02_FrameSE02.Screen02_FrameSE02" "/Game/SciFiScreenConstructor/Meshes/Screen02_FrameSE01.Screen02_FrameSE01"))
  (bind _returnvalue_17 (select _illumination1_2 "/Game/SciFiScreenConstructor/Meshes/Screen02_FrameSE02.Screen02_FrameSE02" "/Game/SciFiScreenConstructor/Meshes/Screen02_FrameSE01.Screen02_FrameSE01"))
  (bind _returnvalue_18 (select _illumination2_2 "/Game/SciFiScreenConstructor/Meshes/Screen02_FrameS02.Screen02_FrameS02" "/Game/SciFiScreenConstructor/Meshes/Screen02_FrameS01.Screen02_FrameS01"))
  (bind _returnvalue_19 (/ _returnvalue_5 4e+01))
  (bind _returnvalue_20 (+ _returnvalue_7 53.0))
  (bind _returnvalue_21 (+ _returnvalue_8 -8.0))
  (bind _returnvalue_22 (select _returnvalue 7e+01 0.0))
  (bind _returnvalue_23 (Math|Float|Floor _returnvalue_19))
  (bind _returnvalue_24 (Math|Float|Fraction _returnvalue_19))
  (bind _returnvalue_25 (select _returnvalue_2 4e+01 _returnvalue_22))
  (bind _returnvalue_26 (< _returnvalue_24 0.5))
  (bind _returnvalue_27 (* _returnvalue_24 4e+01))
  (bind _returnvalue_28 (select _returnvalue_3 2e+01 _returnvalue_25))
  (bind _returnvalue_29 (+ _returnvalue_4 _returnvalue_28))
  (bind _returnvalue_30 (select _returnvalue_26 _returnvalue_27 2e+01))
  (bind _returnvalue_31 (- -25.0 _returnvalue_30))
  (bind _returnvalue_32 (+ _returnvalue_29 -2e+01))
  (if (and (== (Variables|Default|GetLengthLeft) -1) (== (Variables|Default|GetLengthRight) -1))
    (Variables|Default|SetLengthRight 0))
  (if (<= (Variables|Default|GetAngle) 1.0)
    (Components|DestroyComponent (Variables|Default|GetComponentB2)))
  (Components|StaticMesh|SetStaticMesh (Variables|Default|GetComponentG1) (Utilities|Select :Index (Variables|Default|GetGrille1) :Option%200 "/Game/SciFiScreenConstructor/Meshes/Screen02_Grille01.Screen02_Grille01" :Option%201 "/Game/SciFiScreenConstructor/Meshes/Screen02_Grille02.Screen02_Grille02" :Option%202 "/Game/SciFiScreenConstructor/Meshes/Screen02_Grille03.Screen02_Grille03" :Option%203 "/Game/SciFiScreenConstructor/Meshes/Screen02_Grille04.Screen02_Grille04"))
  (Components|StaticMesh|SetStaticMesh (Variables|Default|GetComponentG2) (Utilities|Select :Index (Variables|Default|GetGrille2) :Option%200 "/Game/SciFiScreenConstructor/Meshes/Screen02_Grille01.Screen02_Grille01" :Option%201 "/Game/SciFiScreenConstructor/Meshes/Screen02_Grille02.Screen02_Grille02" :Option%202 "/Game/SciFiScreenConstructor/Meshes/Screen02_Grille03.Screen02_Grille03" :Option%203 "/Game/SciFiScreenConstructor/Meshes/Screen02_Grille04.Screen02_Grille04"))
  (Components|StaticMesh|SetStaticMesh (Variables|Default|GetComponentEL1) _returnvalue_17)
  (Components|StaticMesh|SetStaticMesh (Variables|Default|GetComponentER1) _returnvalue_17)
  (Components|StaticMesh|SetStaticMesh (Variables|Default|GetComponentEL2) _returnvalue_16)
  (Components|StaticMesh|SetStaticMesh (Variables|Default|GetComponentER2) _returnvalue_16)
  (Transformation|SetRelativeRotation (Variables|Default|GetRootMovable) (Math|Rotator|MakeRotator (Variables|Default|GetAngle) 0.0 0.0) false false)
  (Transformation|SetRelativeLocation (Variables|Default|GetFrame) (Math|Vector|MakeVector (- -8.0 (* _width_2 (Variables|Default|GetOffset))) -8.0 -1.0) false false)
  (Transformation|SetRelativeLocation (Variables|Default|GetComponent2) (Math|Vector|MakeVector -5.0 (- -37.0 _width_2) 12.0) false false)
  (for _index (range 0 (Math|Float|Floor (/ (+ (* _width_4 (- 1.0 _offset)) -3.5) 4e+01)))
    (bind _returnvalue_33 (AddComponent|AddStaticMeshComponent false (Math|Transform|MakeTransform (Math|Vector|MakeVector 0.0 (- -29.0 (* _index 4e+01)) -6.0) "0, 0, 0" "1.000000,1.000000,1.000000")))
    (Transformation|AttachComponentToComponent _returnvalue_33 (Variables|Default|GetComponent2) "None" "KeepRelative" "KeepRelative" "KeepRelative" true))
  (for _index_2 (range 0 (Math|Float|Floor (/ (+ (* _width_4 _offset) -3.5) 4e+01)))
    (bind _returnvalue_34 (AddComponent|AddStaticMeshComponent false (Math|Transform|MakeTransform (Math|Vector|MakeVector 0.0 (- -29.0 (* _index_2 4e+01)) -6.0) "0, 0, 0" "1.000000,1.000000,1.000000")))
    (Transformation|AttachComponentToComponent _returnvalue_34 (Variables|Default|GetComponent1) "None" "KeepRelative" "KeepRelative" "KeepRelative" true))
  (Transformation|SetRelativeLocation (Variables|Default|GetComponentEL1) (Math|Vector|MakeVector (* _returnvalue_32 -1.0) 0.0 2.0) false false)
  (Transformation|SetRelativeLocation (Variables|Default|GetComponentER1) (Math|Vector|MakeVector (+ (+ (* (Variables|Default|GetLengthRight) 4e+01) (select (== (Variables|Default|GetLengthRight) 1) 2e+01 (select (== (Variables|Default|GetLengthRight) 0) 4e+01 (select (== (Variables|Default|GetLengthRight) -1) 7e+01 0.0)))) -2e+01) 0.0 2.0) false false)
  (Transformation|SetRelativeLocation (Variables|Default|GetComponentEL2) (Math|Vector|MakeVector _returnvalue_32 0.0 2.0) false false)
  (Transformation|SetRelativeLocation (Variables|Default|GetComponentER2) (Math|Vector|MakeVector (* (+ (+ (* (Variables|Default|GetLengthRight) 4e+01) (select (== (Variables|Default|GetLengthRight) 1) 2e+01 (select (== (Variables|Default|GetLengthRight) 0) 4e+01 (select (== (Variables|Default|GetLengthRight) -1) 7e+01 0.0)))) -2e+01) -1.0) 0.0 2.0) false false)
  (Components|StaticMesh|SetStaticMesh (Variables|Default|GetComponentFan1) (select (Variables|Default|GetFan1) "/Game/SciFiScreenConstructor/Meshes/Screen02_Fan01.Screen02_Fan01" "/Game/SciFiScreenConstructor/Meshes/Screen02_Fan02.Screen02_Fan02"))
  (Components|StaticMesh|SetStaticMesh (Variables|Default|GetComponentFan2) (select (Variables|Default|GetFan2) "/Game/SciFiScreenConstructor/Meshes/Screen02_Fan01.Screen02_Fan01" "/Game/SciFiScreenConstructor/Meshes/Screen02_Fan02.Screen02_Fan02"))
  (Transformation|SetRelativeTransform _componentscreen (Math|Transform|MakeTransform (Math|Vector|MakeVector (+ (* (- _returnvalue_32 (+ (+ (* (Variables|Default|GetLengthRight) 4e+01) (select (== (Variables|Default|GetLengthRight) 1) 2e+01 (select (== (Variables|Default|GetLengthRight) 0) 4e+01 (select (== (Variables|Default|GetLengthRight) -1) 7e+01 0.0)))) -2e+01)) -0.5) -5.0) _returnvalue_21 14.0) "0, 0, 0" (* (Math|Vector|MakeVector (+ (+ _returnvalue_32 (+ (+ (* (Variables|Default|GetLengthRight) 4e+01) (select (== (Variables|Default|GetLengthRight) 1) 2e+01 (select (== (Variables|Default|GetLengthRight) 0) 4e+01 (select (== (Variables|Default|GetLengthRight) -1) 7e+01 0.0)))) -2e+01)) 4.0) _returnvalue_20 1e+02) 0.01)) false false)
  (Transformation|SetRelativeTransform (Variables|Default|GetComponentScreenB) (Math|Transform|MakeTransform (Math|Vector|MakeVector (+ (* (- _returnvalue_32 (+ (+ (* (Variables|Default|GetLengthRight) 4e+01) (select (== (Variables|Default|GetLengthRight) 1) 2e+01 (select (== (Variables|Default|GetLengthRight) 0) 4e+01 (select (== (Variables|Default|GetLengthRight) -1) 7e+01 0.0)))) -2e+01)) -0.5) -5.0) _returnvalue_21 14.0) (Math|Rotator|MakeRotator (select _screenbacksideflipx 1.8e+02 0.0) (select _screenbacksideflipy 1.8e+02 0.0) 0.0) (* (Math|Vector|MakeVector (+ (+ _returnvalue_32 (+ (+ (* (Variables|Default|GetLengthRight) 4e+01) (select (== (Variables|Default|GetLengthRight) 1) 2e+01 (select (== (Variables|Default|GetLengthRight) 0) 4e+01 (select (== (Variables|Default|GetLengthRight) -1) 7e+01 0.0)))) -2e+01)) 4.0) _returnvalue_20 (select (Class|KismetMathLibrary|XORBoolean _screenbacksideflipx _screenbacksideflipy) 1e+02 -1e+02)) 0.01)) false false)
  (if (Variables|Default|GetScreenStretch)
    (Rendering|Material|SetMaterial _componentscreen 0 _displaymaterial)
    (else
      (bind _returnvalue_35 (Rendering|Material|CreateDynamicMaterialInstance _componentscreen 0 _displaymaterial "None" :!class /Script/Engine.PrimitiveComponent))
      (Rendering|Material|SetMaterial (Variables|Default|GetComponentScreenB) 0 _returnvalue_35)
      (Rendering|Material|SetVectorParameterValue _returnvalue_35 "UVmultiplyUVadd" (Utilities|Struct|MakeLinearColor (select (Class|KismetMathLibrary|XORBoolean (> (+ (+ _returnvalue_32 (+ (+ (* (Variables|Default|GetLengthRight) 4e+01) (select (== (Variables|Default|GetLengthRight) 1) 2e+01 (select (== (Variables|Default|GetLengthRight) 0) 4e+01 (select (== (Variables|Default|GetLengthRight) -1) 7e+01 0.0)))) -2e+01)) 4.0) _returnvalue_20) (Variables|Default|GetScreenTiling)) 1.0 (/ (+ (+ _returnvalue_32 (+ (+ (* (Variables|Default|GetLengthRight) 4e+01) (select (== (Variables|Default|GetLengthRight) 1) 2e+01 (select (== (Variables|Default|GetLengthRight) 0) 4e+01 (select (== (Variables|Default|GetLengthRight) -1) 7e+01 0.0)))) -2e+01)) 4.0) _returnvalue_20)) (select (Class|KismetMathLibrary|XORBoolean (> (+ (+ _returnvalue_32 (+ (+ (* (Variables|Default|GetLengthRight) 4e+01) (select (== (Variables|Default|GetLengthRight) 1) 2e+01 (select (== (Variables|Default|GetLengthRight) 0) 4e+01 (select (== (Variables|Default|GetLengthRight) -1) 7e+01 0.0)))) -2e+01)) 4.0) _returnvalue_20) (Variables|Default|GetScreenTiling)) (/ _returnvalue_20 (+ (+ _returnvalue_32 (+ (+ (* (Variables|Default|GetLengthRight) 4e+01) (select (== (Variables|Default|GetLengthRight) 1) 2e+01 (select (== (Variables|Default|GetLengthRight) 0) 4e+01 (select (== (Variables|Default|GetLengthRight) -1) 7e+01 0.0)))) -2e+01)) 4.0)) 1.0) (* (- (select (Class|KismetMathLibrary|XORBoolean (> (+ (+ _returnvalue_32 (+ (+ (* (Variables|Default|GetLengthRight) 4e+01) (select (== (Variables|Default|GetLengthRight) 1) 2e+01 (select (== (Variables|Default|GetLengthRight) 0) 4e+01 (select (== (Variables|Default|GetLengthRight) -1) 7e+01 0.0)))) -2e+01)) 4.0) _returnvalue_20) (Variables|Default|GetScreenTiling)) 1.0 (/ (+ (+ _returnvalue_32 (+ (+ (* (Variables|Default|GetLengthRight) 4e+01) (select (== (Variables|Default|GetLengthRight) 1) 2e+01 (select (== (Variables|Default|GetLengthRight) 0) 4e+01 (select (== (Variables|Default|GetLengthRight) -1) 7e+01 0.0)))) -2e+01)) 4.0) _returnvalue_20)) 1.0) _returnvalue_6) (* (- (select (Class|KismetMathLibrary|XORBoolean (> (+ (+ _returnvalue_32 (+ (+ (* (Variables|Default|GetLengthRight) 4e+01) (select (== (Variables|Default|GetLengthRight) 1) 2e+01 (select (== (Variables|Default|GetLengthRight) 0) 4e+01 (select (== (Variables|Default|GetLengthRight) -1) 7e+01 0.0)))) -2e+01)) 4.0) _returnvalue_20) (Variables|Default|GetScreenTiling)) (/ _returnvalue_20 (+ (+ _returnvalue_32 (+ (+ (* (Variables|Default|GetLengthRight) 4e+01) (select (== (Variables|Default|GetLengthRight) 1) 2e+01 (select (== (Variables|Default|GetLengthRight) 0) 4e+01 (select (== (Variables|Default|GetLengthRight) -1) 7e+01 0.0)))) -2e+01)) 4.0)) 1.0) 1.0) _returnvalue_6)) :!class /Script/Engine.MaterialInstanceDynamic)))
  (Utilities|FlowControl|Sequence
    (:then_0
      (switch int (Variables|Default|GetLengthRight)
        (:Default
          (Components|StaticMesh|SetStaticMesh (Variables|Default|GetComponentFCTR1) _returnvalue_15)
          (Components|StaticMesh|SetStaticMesh (Variables|Default|GetComponentFCTR2) _returnvalue_13)
          (for _index_3 (range 1 (- (Variables|Default|GetLengthRight) 1))
            (bind _returnvalue_36 (AddComponent|AddStaticMeshComponent false (Math|Transform|MakeTransform (Math|Vector|MakeVector (* _index_3 -4e+01) _returnvalue_31 -4.0) "0, 0, 0" "1.000000,1.000000,1.000000")))
            (Transformation|AttachComponentToComponent _returnvalue_36 _component2 "None" "KeepRelative" "KeepRelative" "KeepRelative" true)
            (for _index_4 (range 1 _returnvalue_23)
              (bind _returnvalue_37 (AddComponent|AddStaticMeshComponent false (Math|Transform|MakeTransform (Math|Vector|MakeVector 0.0 (* _index_4 -4e+01) 0.0) "0, 0, 0" "1.000000,1.000000,1.000000")))
              (Transformation|AttachComponentToComponent _returnvalue_37 _returnvalue_36 "None" "KeepRelative" "KeepRelative" "KeepRelative" true)))
          (for _index_5 (range 2 (- (Variables|Default|GetLengthRight) 1))
            (bind _returnvalue_38 (AddComponent|AddStaticMeshComponent false (Math|Transform|MakeTransform (Math|Vector|MakeVector (* _index_5 4e+01) 0.0 2.0) "0, 0, 0" "1.000000,1.000000,1.000000")))
            (Transformation|AttachComponentToComponent _returnvalue_38 (Variables|Default|GetComponent1) "None" "KeepRelative" "KeepRelative" "KeepRelative" true)
            (Components|StaticMesh|SetStaticMesh _returnvalue_38 _returnvalue_11)
            (bind _returnvalue_39 (AddComponent|AddStaticMeshComponent false (Math|Transform|MakeTransform (Math|Vector|MakeVector (* (* _index_5 4e+01) -1.0) 0.0 2.0) "0, 0, 0" "1.000000,1.000000,1.000000")))
            (Transformation|AttachComponentToComponent _returnvalue_39 (Variables|Default|GetComponent2) "None" "KeepRelative" "KeepRelative" "KeepRelative" true)
            (Components|StaticMesh|SetStaticMesh _returnvalue_39 _returnvalue_18)))
        (:-1
          (Components|StaticMesh|SetStaticMesh (Variables|Default|GetComponentFC1) "/Game/SciFiScreenConstructor/Meshes/Screen02_FrameCS01.Screen02_FrameCS01")
          (Components|StaticMesh|SetStaticMesh (Variables|Default|GetComponentFC2) "/Game/SciFiScreenConstructor/Meshes/Screen02_FrameCS02.Screen02_FrameCS02")
          (Components|StaticMesh|SetStaticMesh _componentg1_2 _returnvalue_12)
          (Transformation|SetRelativeLocationAndRotation _componentg1_2 "-5.000000,1.000000,2.000000" "0,180.000000, 0" false false)
          (Components|StaticMesh|SetStaticMesh _componentg2_2 _returnvalue_9)
          (Transformation|SetRelativeLocationAndRotation _componentg2_2 "5.000000,1.000000,2.000000" "0, 0, 0" false false)
          (Components|StaticMesh|SetStaticMesh (Variables|Default|GetComponentER1) "/Game/SciFiScreenConstructor/Meshes/Screen02_FrameCE01.Screen02_FrameCE01" :!label _label)
          (Components|StaticMesh|SetStaticMesh (Variables|Default|GetComponentER2) "/Game/SciFiScreenConstructor/Meshes/Screen02_FrameCE01.Screen02_FrameCE01")
          (Components|DestroyComponent (Variables|Default|GetComponentFCTR1)))
        (:0
          (goto _label))
        (:1
          (Components|StaticMesh|SetStaticMesh (Variables|Default|GetComponentFCTR1) _returnvalue_14)
          (Components|StaticMesh|SetStaticMesh (Variables|Default|GetComponentFCTR2) _returnvalue_10))))
    (:then_1
      (switch int (Variables|Default|GetLengthLeft)
        (:Default
          (Components|StaticMesh|SetStaticMesh (Variables|Default|GetComponentFCTL1) _returnvalue_15)
          (Components|StaticMesh|SetStaticMesh (Variables|Default|GetComponentFCTL2) _returnvalue_13)
          (for _index_6 (range 1 (- (Variables|Default|GetLengthLeft) 1))
            (bind _returnvalue_40 (AddComponent|AddStaticMeshComponent false (Math|Transform|MakeTransform (Math|Vector|MakeVector (* _index_6 4e+01) _returnvalue_31 -4.0) "0, 0, 0" "1.000000,1.000000,1.000000")))
            (Transformation|AttachComponentToComponent _returnvalue_40 _component2 "None" "KeepRelative" "KeepRelative" "KeepRelative" true)
            (for _index_7 (range 1 _returnvalue_23)
              (bind _returnvalue_41 (AddComponent|AddStaticMeshComponent false (Math|Transform|MakeTransform (Math|Vector|MakeVector 0.0 (* _index_7 -4e+01) 0.0) "0, 0, 0" "1.000000,1.000000,1.000000")))
              (Transformation|AttachComponentToComponent _returnvalue_41 _returnvalue_40 "None" "KeepRelative" "KeepRelative" "KeepRelative" true)))
          (for _index_8 (range 2 (- (Variables|Default|GetLengthLeft) 1))
            (bind _returnvalue_42 (AddComponent|AddStaticMeshComponent false (Math|Transform|MakeTransform (Math|Vector|MakeVector (* _index_8 4e+01) 0.0 2.0) "0, 0, 0" "1.000000,1.000000,1.000000")))
            (Transformation|AttachComponentToComponent _returnvalue_42 (Variables|Default|GetComponent2) "None" "KeepRelative" "KeepRelative" "KeepRelative" true)
            (Components|StaticMesh|SetStaticMesh _returnvalue_42 _returnvalue_11)
            (bind _returnvalue_43 (AddComponent|AddStaticMeshComponent false (Math|Transform|MakeTransform (Math|Vector|MakeVector (* (* _index_8 4e+01) -1.0) 0.0 2.0) "0, 0, 0" "1.000000,1.000000,1.000000")))
            (Transformation|AttachComponentToComponent _returnvalue_43 (Variables|Default|GetComponent1) "None" "KeepRelative" "KeepRelative" "KeepRelative" true)
            (Components|StaticMesh|SetStaticMesh _returnvalue_43 _returnvalue_18)))
        (:-1
          (Components|StaticMesh|SetStaticMesh (Variables|Default|GetComponentFC1) "/Game/SciFiScreenConstructor/Meshes/Screen02_FrameCS02.Screen02_FrameCS02")
          (Components|StaticMesh|SetStaticMesh (Variables|Default|GetComponentFC2) "/Game/SciFiScreenConstructor/Meshes/Screen02_FrameCS01.Screen02_FrameCS01")
          (Components|StaticMesh|SetStaticMesh _componentg1 _returnvalue_12)
          (Transformation|SetRelativeLocation _componentg1 "5.000000,1.000000,2.000000" false false)
          (Components|StaticMesh|SetStaticMesh _componentg2 _returnvalue_9)
          (Transformation|SetRelativeLocation _componentg2 "-5.000000,1.000000,2.000000" false false)
          (Components|StaticMesh|SetStaticMesh (Variables|Default|GetComponentEL1) "/Game/SciFiScreenConstructor/Meshes/Screen02_FrameCE01.Screen02_FrameCE01" :!label _label_2)
          (Components|StaticMesh|SetStaticMesh (Variables|Default|GetComponentEL2) "/Game/SciFiScreenConstructor/Meshes/Screen02_FrameCE01.Screen02_FrameCE01")
          (Components|DestroyComponent (Variables|Default|GetComponentFCTL1)))
        (:0
          (goto _label_2))
        (:1
          (Components|StaticMesh|SetStaticMesh (Variables|Default|GetComponentFCTL1) _returnvalue_14)
          (Components|StaticMesh|SetStaticMesh (Variables|Default|GetComponentFCTL2) _returnvalue_10))))
    (:then_2
      (for _array_element (Components|GetChildrenComponents (Variables|Default|GetDefaultSceneRoot) true)
        (if (and (!= _array_element (Variables|Default|GetComponentScreen)) (!= _array_element (Variables|Default|GetComponentScreenB)))
          (bind _as静态网格体组件 (Utilities|Casting|CastToStaticMeshComponent _array_element))
          (Rendering|Material|SetMaterial _as静态网格体组件 0 (Variables|Default|GetBaseMaterial)))))))