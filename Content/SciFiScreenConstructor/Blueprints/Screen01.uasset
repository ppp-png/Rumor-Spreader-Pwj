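; Configurable sci-fi screen prop, assembled entirely in the construction script.
; Length scales the front and back screens and spawns repeated frame segments; options set mounting style, tilt, side cases, fan and wires, which replace bottom frames on short screens.
; Unless stretched, both screens share a dynamic material whose UVs correct aspect ratio with tiling and offset.
; The back face supports flips, and all other meshes receive BaseMaterial.
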(event EventBeginPlay)

(event Collision|EventActorBeginOverlap
  (params (OtherActor :type Actor%20Object%20Reference)))

(event EventTick
  (params (DeltaSeconds :type Float%20%28single-precision%29)))

(fn ConstructionScript
  (bind _returnvalue (Math|Float|MakeLiteralFloat 52.0))
  (bind _returnvalue_2 (Math|Float|MakeLiteralFloat 87.0))
  (bind _screentiling (Variables|Default|GetScreenTiling))
  (bind _displaymaterial (Variables|Default|GetDisplayMaterial))
  (bind _length (Variables|Default|GetLength))
  (bind _length_2 (Variables|Default|GetLength))
  (bind _screenbacksideflipy (Variables|Default|GetScreenBackSideFlipY))
  (bind _componentscreen (Variables|Default|GetComponentScreen))
  (bind _sideconstraint (Variables|Default|GetSideConstraint))
  (bind _length_3 (Variables|Default|GetLength))
  (bind _rootmovabler (Variables|Default|GetRootMovableR))
  (bind _screenmaterialoffset (Variables|Default|GetScreenMaterialOffset))
  (bind _screenbacksideflipx (Variables|Default|GetScreenBackSideFlipX))
  (bind _length_4 (Variables|Default|GetLength))
  (bind _eta01 (Variables|Default|GetETA01))
  (bind _angle (Variables|Default|GetAngle))
  (bind _returnvalue_3 (* _length_3 _returnvalue))
  (bind _returnvalue_4 (* _screenmaterialoffset -1.0))
  (bind _returnvalue_5 (+ _length_4 -1))
  (bind _returnvalue_6 (* _angle -1.0))
  (bind _returnvalue_7 (* _returnvalue_5 -52.0))
  (bind _returnvalue_8 (+ _returnvalue_3 4.0))
  (bind _returnvalue_9 (Math|Vector|MakeVector _returnvalue_7 0.0 0.0))
  (bind _returnvalue_10 (/ _returnvalue_2 _returnvalue_8))
  (bind _returnvalue_11 (/ _returnvalue_8 _returnvalue_2))
  (bind _returnvalue_12 (> _returnvalue_8 _returnvalue_2))
  (bind _returnvalue_13 (* _returnvalue_8 -0.5))
  (bind _returnvalue_14 (Class|KismetMathLibrary|XORBoolean _returnvalue_12 _screentiling))
  (bind _returnvalue_15 (+ _returnvalue_13 -2.0))
  (bind _returnvalue_16 (select _returnvalue_14 1.0 _returnvalue_11))
  (bind _returnvalue_17 (select _returnvalue_14 _returnvalue_10 1.0))
  (Transformation|SetRelativeTransform (Variables|Default|GetComponentScreen) (Math|Transform|MakeTransform (Math|Vector|MakeVector _returnvalue_15 0.0 0.0) "0, 0, 0" (* (Math|Vector|MakeVector _returnvalue_8 _returnvalue_2 1e+02) 0.01)) false false)
  (Transformation|SetRelativeTransform (Variables|Default|GetComponentScreenB) (Math|Transform|MakeTransform (Math|Vector|MakeVector _returnvalue_15 0.0 0.0) (Math|Rotator|MakeRotator (select _screenbacksideflipy 1.8e+02 0.0) (select _screenbacksideflipx 1.8e+02 0.0) 0.0) (* (Math|Vector|MakeVector _returnvalue_8 _returnvalue_2 (select (Class|KismetMathLibrary|XORBoolean _screenbacksideflipy _screenbacksideflipx) 1e+02 -1e+02)) 0.01)) false false)
  (if (Variables|Default|GetScreenStretch)
    (Rendering|Material|SetMaterial _componentscreen 0 _displaymaterial)
    (else
      (bind _returnvalue_18 (Rendering|Material|CreateDynamicMaterialInstance _componentscreen 0 _displaymaterial "None" :!class /Script/Engine.PrimitiveComponent))
      (Rendering|Material|SetVectorParameterValue _returnvalue_18 "UVmultiplyUVadd" (Utilities|Struct|MakeLinearColor _returnvalue_16 _returnvalue_17 (* (- _returnvalue_16 1.0) _returnvalue_4) (* (- _returnvalue_17 1.0) _returnvalue_4)) :!class /Script/Engine.MaterialInstanceDynamic)
      (Rendering|Material|SetMaterial (Variables|Default|GetComponentScreenB) 0 _returnvalue_18)))
  (Components|StaticMesh|SetStaticMesh (Variables|Default|GetRootR) (select _sideconstraint "/Game/SciFiScreenConstructor/Meshes/Screen01_Base2.Screen01_Base2" "/Game/SciFiScreenConstructor/Meshes/Screen01_Base1.Screen01_Base1"))
  (Components|StaticMesh|SetStaticMesh (Variables|Default|GetRootMovableR) (select _sideconstraint "/Game/SciFiScreenConstructor/Meshes/Screen01_BaseF2.Screen01_BaseF2" "/Game/SciFiScreenConstructor/Meshes/Screen01_BaseF1.Screen01_BaseF1"))
  (Components|StaticMesh|SetStaticMesh (Variables|Default|GetRootMovableL) (select _sideconstraint "/Game/SciFiScreenConstructor/Meshes/Screen01_BaseF2a.Screen01_BaseF2a" "/Game/SciFiScreenConstructor/Meshes/Screen01_BaseF1a.Screen01_BaseF1a"))
  (Transformation|SetRelativeRotation (Variables|Default|GetRootMovableR) (select (Variables|Default|GetSideConstraint) (Math|Rotator|MakeRotator 0.0 _returnvalue_6 0.0) (Math|Rotator|MakeRotator _returnvalue_6 0.0 0.0)) false false)
  (if (Variables|Default|GetSideConstraint)
    (Components|DestroyComponent (Variables|Default|GetRootL))
    (else
      (Transformation|SetRelativeLocation (Variables|Default|GetRootL) (+ _returnvalue_9 (Utilities|Array|Get(acopy) _eta01)) false false)))
  (Transformation|SetRelativeLocation (Variables|Default|GetRootMovableL) (+ _returnvalue_9 (Utilities|Array|Get(acopy) _eta01 1)) false false)
  (for _index (range 1 (Variables|Default|GetLength))
    (bind _returnvalue_19 (AddComponent|AddStaticMeshComponent false (Math|Transform|MakeTransform (Math|Vector|MakeVector (+ (* (+ _index -1) -52.0) -45.0) 0.0 3.0) "0, 0, 0" "1.000000,1.000000,1.000000")))
    (Transformation|AttachComponentToComponent _returnvalue_19 _rootmovabler "None" "KeepRelative" "KeepRelative" "KeepRelative" true)
    (Components|StaticMesh|SetStaticMesh _returnvalue_19 "/Game/SciFiScreenConstructor/Meshes/Screen01_FrameT.Screen01_FrameT")
    (if (not (Math|Boolean|ANDBoolean (>= _length_2 1) (<= _length_2 3) (Variables|Default|GetWires)))
      (bind _returnvalue_20 (AddComponent|AddStaticMeshComponent false (Math|Transform|MakeTransform (Math|Vector|MakeVector (+ (* (+ _index -1) -52.0) -45.0) 103.0 3.0) "0, 0, 0" "1.000000,1.000000,1.000000")))
      (Transformation|AttachComponentToComponent _returnvalue_20 _rootmovabler "None" "KeepRelative" "KeepRelative" "KeepRelative" true)
      (Components|StaticMesh|SetStaticMesh _returnvalue_20 "/Game/SciFiScreenConstructor/Meshes/Screen01_FrameB.Screen01_FrameB")))
  (Components|StaticMesh|SetStaticMesh (Variables|Default|GetComponent02L) (select (Variables|Default|GetLeftCase) "/Game/SciFiScreenConstructor/Meshes/Screen01_FrameLC.Screen01_FrameLC" "/Game/SciFiScreenConstructor/Meshes/Screen01_FrameLU.Screen01_FrameLU"))
  (Components|StaticMesh|SetStaticMesh (Variables|Default|GetComponent02R) (select (Variables|Default|GetRightCase) "/Game/SciFiScreenConstructor/Meshes/Screen01_FrameRC.Screen01_FrameRC" "/Game/SciFiScreenConstructor/Meshes/Screen01_FrameRU.Screen01_FrameRU"))
  (Components|StaticMesh|SetStaticMesh (Variables|Default|GetComponentFan) (select (Variables|Default|GetFan) "/Game/SciFiScreenConstructor/Meshes/Screen01_Fan2.Screen01_Fan2" "/Game/SciFiScreenConstructor/Meshes/Screen01_Fan1.Screen01_Fan1"))
  (if (Math|Boolean|ANDBoolean (>= _length 1) (<= _length 3) (Variables|Default|GetWires))
    (Components|DestroyComponent (Variables|Default|GetComponentWiresL))
    (Components|StaticMesh|SetStaticMesh (Variables|Default|GetComponentWiresBase) "/Game/SciFiScreenConstructor/Meshes/Screen01_Wire0.Screen01_Wire0")
    (Components|StaticMesh|SetStaticMesh (Variables|Default|GetComponentWiresR) (Utilities|Select :Index (+ (Variables|Default|GetLength) -1) :Option%200 "/Game/SciFiScreenConstructor/Meshes/Screen01_Wire1.Screen01_Wire1" :Option%201 "/Game/SciFiScreenConstructor/Meshes/Screen01_Wire2.Screen01_Wire2" :Option%202 "/Game/SciFiScreenConstructor/Meshes/Screen01_Wire3.Screen01_Wire3"))
    (else
      (Components|DestroyComponent (Variables|Default|GetComponentWiresR))))
  (for _array_element (Components|GetChildrenComponents (Variables|Default|GetDefaultSceneRoot) true)
    (if (and (!= _array_element (Variables|Default|GetComponentScreen)) (!= _array_element (Variables|Default|GetComponentScreenB)))
      (bind _as静态网格体组件 (Utilities|Casting|CastToStaticMeshComponent _array_element))
      (Rendering|Material|SetMaterial _as静态网格体组件 0 (Variables|Default|GetBaseMaterial)))))